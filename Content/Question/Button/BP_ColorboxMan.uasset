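; BP_ColorboxMan manages a four-cube code puzzle, checking the order in which Cube1 to Cube4 are hit.
; On BeginPlay it binds each cube's hit event, and each hit appends that cube's ID to an input array.
; The fourth input packs the IDs into a four-digit integer compared against CorrectAnswer.
; A match fires AnswerRight; a mismatch fires AnswerWrong and resets the cubes and input for another attempt.
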(event `self.ReceiveBeginPlay`
  (add `/Game/Question/Button/PasswardButton.OnCubeHit` (`self.Cube1`) (delegate `OnHitCube1`))
  (add `/Game/Question/Button/PasswardButton.OnCubeHit` (`self.Cube2`) (delegate `OnHitCube2`))
  (add `/Game/Question/Button/PasswardButton.OnCubeHit` (`self.Cube3`) (delegate `OnHitCube3`))
  (add `/Game/Question/Button/PasswardButton.OnCubeHit` (`self.Cube4`) (delegate `OnHitCube4`)))

(event `OnHitCube2`
  (`self.AddUserInput` 2))

(event `OnHitCube4`
  (`self.AddUserInput` 4))

(event `OnHitCube3`
  (`self.AddUserInput` 3))

(event `OnHitCube1`
  (`self.AddUserInput` 1))

(fn `AddUserInput`
  (params (CubeID :type Integer))
  (`KismetArrayLibrary.Array_Set` (`self.arUserInput`) (`self.nIndex`) CubeID true)
  (bind _output_get (set `self.nIndex` (+ 1 (`self.nIndex`))))
  (if (== _output_get 4)
    (`KismetSystemLibrary.PrintString` "4 check")
    (bind _return_value (`self.Make 4Digit`))
    (if (== _return_value (`self.CorrectAnswer`))
      (`self.OnAnswerRight`)
      (else
        (`self.OnAnswerWrong`)
        (`/Game/Question/Button/PasswardButton.ResetData` (`self.Cube1`))
        (`/Game/Question/Button/PasswardButton.ResetData` (`self.Cube2`))
        (`/Game/Question/Button/PasswardButton.ResetData` (`self.Cube3`))
        (`/Game/Question/Button/PasswardButton.ResetData` (`self.Cube4`))
        (`KismetArrayLibrary.Array_Set` (`self.arUserInput`) 0 -1)
        (`KismetArrayLibrary.Array_Set` (`self.arUserInput`) 1 -1)
        (`KismetArrayLibrary.Array_Set` (`self.arUserInput`) 2 -1)
        (`KismetArrayLibrary.Array_Set` (`self.arUserInput`) 3 -1)
        (set `self.nIndex` 0)))))

(fn `Make 4Digit`
  (returns (`Return Value` :type Integer))
  (bind _returnvalue (+ (* (`|GetArrayItem` (`self.arUserInput`)) 1000) (* (`|GetArrayItem` (`self.arUserInput`) 1) 100) (* (`|GetArrayItem` (`self.arUserInput`) 2) 10) (`|GetArrayItem` (`self.arUserInput`) 3)))
  (`KismetSystemLibrary.PrintString` (`KismetStringLibrary.Conv_IntToString` _returnvalue))
  (return _returnvalue))

(fn `UserConstructionScript`)